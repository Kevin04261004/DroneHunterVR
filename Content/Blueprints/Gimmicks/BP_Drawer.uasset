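; VR drawer gimmick that slides along its forward axis as the player's hand pulls or pushes it.
; BP_GrabComponent events toggle the grabbed state and record the motion controller's starting position.
; While grabbed, Tick dots the controller's per-frame movement with the forward vector and applies it as a local X offset, without travel limits.
; Two unconnected alternatives remain, using projected world-space deltas from the previous frame or initial grab.
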(event `self.ReceiveTick`
  (params (DeltaSeconds :type "Float (single-precision)"))
  (bind _grabbinghand (`/Game/Blueprints/BP_GrabComponent.GrabbingHand` (`self.BP_GrabComponent`)))
  (bind _returnvalue (`SceneComponent.K2_GetComponentLocation` (`/Game/Blueprints/BP_Hand.MotionController` _grabbinghand)))
  ;[1 1 1] Local 좌표를 이용하는 방법
  (if (`self.Grabbed`)
    (`/Engine/EditorBlueprintResources/StandardMacros.IsValid` _grabbinghand
      (:`Is Valid`
        (`self.K2_AddActorLocalOffset` (`KismetMathLibrary.MakeVector` (`KismetMathLibrary.Dot_VectorVector` (- _returnvalue (`self.PrevMCGrabLocation`)) (`self.GetActorForwardVector`))))
        (set `self.PrevMCGrabLocation` _returnvalue)))))

(event `self.BP_GrabComponent.OnGrabbed`
  (bind _grabbinghand (`/Game/Blueprints/BP_GrabComponent.GrabbingHand` (`self.BP_GrabComponent`)))
  (`/Engine/EditorBlueprintResources/StandardMacros.IsValid` _grabbinghand
    (:`Is Valid`
      (bind _output_get (set `self.MCGrabLocation` (`SceneComponent.K2_GetComponentLocation` (`/Game/Blueprints/BP_Hand.MotionController` _grabbinghand))))
      (set `self.PrevMCGrabLocation` _output_get)
      (set `self.ActorGrabLocation` (`self.K2_GetActorLocation`))
      (set `self.Grabbed` true))))

(event `self.BP_GrabComponent.OnDropped`
  (`/Engine/EditorBlueprintResources/StandardMacros.IsValid` (`/Game/Blueprints/BP_GrabComponent.GrabbingHand` (`self.BP_GrabComponent`))
    (:`Is Valid`
      (set `self.Grabbed` false))))

(fn `UserConstructionScript`)