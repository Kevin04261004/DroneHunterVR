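; VR lever gimmick that a motion controller can grab and swing around the actor's right axis.
; On grab, BP_GrabComponent events store the controller location and the lever's starting pitch.
; While held, Tick projects start and current hand offsets onto the swing plane, signs their angle with cross and dot products, and adds it to that pitch.
; An unconnected incremental, frame-to-frame variant of this rotation remains in the graph.
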(event `self.ReceiveTick`
  (params (DeltaSeconds :type "Float (single-precision)"))
  (bind _grabbinghand (`/Game/Blueprints/BP_GrabComponent.GrabbingHand` (`self.BP_GrabComponent`)))
  (bind _returnvalue (`KismetMathLibrary.ProjectVectorOnToPlane` (- (`self.MCGrabLocation`) (`self.K2_GetActorLocation`)) (`self.GetActorRightVector`)))
  (bind _returnvalue_2 (`KismetMathLibrary.ProjectVectorOnToPlane` (- (`SceneComponent.K2_GetComponentLocation` (`/Game/Blueprints/BP_Hand.MotionController` _grabbinghand)) (`self.K2_GetActorLocation`)) (`self.GetActorRightVector`)))
  (bind _returnvalue_3 (`KismetMathLibrary.Abs` (`/Game/Blueprints/BP_HelperFunc.GetDegreeBetweenTwoVectors` _returnvalue_2 _returnvalue)))
  (if (`self.Grabbed`)
    (`/Engine/EditorBlueprintResources/StandardMacros.IsValid` _grabbinghand
      (:`Is Valid`
        (if (> (`KismetMathLibrary.Dot_VectorVector` (`KismetMathLibrary.Cross_VectorVector` _returnvalue_2 _returnvalue) (`self.GetActorRightVector`)) 0.0)
          (`SceneComponent.K2_SetRelativeRotation` (`self.Lever`) (`KismetMathLibrary.MakeRotator` 0.0 (+ (`self.LeverGrabRelativeRotY`) _returnvalue_3)) false true)
          (else
            (`SceneComponent.K2_SetRelativeRotation` (`self.Lever`) (`KismetMathLibrary.MakeRotator` 0.0 (+ (`self.LeverGrabRelativeRotY`) (* _returnvalue_3 -1.0))) false true)))))))

(event `self.BP_GrabComponent.OnGrabbed`
  (bind (_relativerotation_roll _relativerotation_pitch) (`KismetMathLibrary.BreakRotator` (`SceneComponent.RelativeRotation` (`self.Lever`))))
  (bind _grabbinghand (`/Game/Blueprints/BP_GrabComponent.GrabbingHand` (`self.BP_GrabComponent`)))
  (`/Engine/EditorBlueprintResources/StandardMacros.IsValid` _grabbinghand
    (:`Is Valid`
      (bind _output_get (set `self.MCGrabLocation` (`SceneComponent.K2_GetComponentLocation` (`/Game/Blueprints/BP_Hand.MotionController` _grabbinghand))))
      (set `self.PrevMCGrabLocation` _output_get)
      (bind _output_get_2 (set `self.LeverGrabRelativeRotY` _relativerotation_pitch))
      (set `self.Grabbed` true)
      (set `self.PrevLeverGrabRelativeRotation` _output_get_2))))

(event `self.BP_GrabComponent.OnDropped`
  (`/Engine/EditorBlueprintResources/StandardMacros.IsValid` (`/Game/Blueprints/BP_GrabComponent.GrabbingHand` (`self.BP_GrabComponent`))
    (:`Is Valid`
      (set `self.Grabbed` false))))

(fn `UserConstructionScript`)