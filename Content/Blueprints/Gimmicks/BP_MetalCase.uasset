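; BP_MetalCase is a VR gimmick: a metal case unlocked by grabbing and twisting its key.
; A state (Closed, Waiting Key Interaction, Open) toggles key visibility and trigger collisions, starting at Waiting Key Interaction.
; While grabbed, the key's pitch follows the motion controller's roll change, and a quarter turn sets Open.
; Tick then plays a one-shot timeline that swings the cover socket open.
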(event `self.ReceiveBeginPlay`
  (bind (_relativerotation_roll _relativerotation_pitch) (`KismetMathLibrary.BreakRotator` (`SceneComponent.RelativeRotation` (`self.MeshKey`))))
  (`self.SetMetalCaseState` "NewEnumerator1")
  (set `self.InitKeyPitch` _relativerotation_pitch))

(event `self.ReceiveTick`
  (params (DeltaSeconds :type "Float (single-precision)"))
  (switch `/Game/Blueprints/Gimmicks/EMetalCase` (`self.State`)
    (:`NewEnumerator1`
      (`self.RotateKey`))
    (:`NewEnumerator2`
      (`/Engine/EditorBlueprintResources/StandardMacros.DoOnce` false
        (:`Completed`
          (bind (_direction _ratio) (`Timeline|CoverOpenTimeline`)
            (:`Update`
              (`SceneComponent.K2_SetRelativeRotation` (`self.CoverSocket`) (`KismetMathLibrary.MakeRotator` (`KismetMathLibrary.Lerp` 0.0 -30.0 _ratio)) false false))))))))

(event `self.BP_GrabComponent.OnGrabbed`
  (bind _relativerotation_roll (`KismetMathLibrary.BreakRotator` (`SceneComponent.RelativeRotation` (`/Game/Blueprints/BP_Hand.MotionController` (`/Game/Blueprints/BP_GrabComponent.GrabbingHand` (`self.BP_GrabComponent`))))))
  (set `self.KeyRelativeRot` (`SceneComponent.RelativeRotation` (`self.MeshKey`)))
  (set `self.MCRelativeRotX` _relativerotation_roll)
  (set `self.GrabbedKey` true))

(event `self.BP_GrabComponent.OnDropped`
  (set `self.GrabbedKey` false))

(fn `OpenCover`)

(fn `RotateKey`
  (bind _meshkey (`self.MeshKey`))
  (bind (_relativerotation_roll _relativerotation_pitch) (`KismetMathLibrary.BreakRotator` (`SceneComponent.RelativeRotation` _meshkey)))
  (bind _relativerotation_roll_2 (`KismetMathLibrary.BreakRotator` (`SceneComponent.RelativeRotation` (`/Game/Blueprints/BP_Hand.MotionController` (`/Game/Blueprints/BP_GrabComponent.GrabbingHand` (`self.BP_GrabComponent`))))))
  (if (`self.GrabbedKey`)
    (`SceneComponent.K2_SetRelativeRotation` _meshkey (`KismetMathLibrary.ComposeRotators` (`self.KeyRelativeRot`) (`KismetMathLibrary.MakeRotator` 0.0 (- (`self.MCRelativeRotX`) _relativerotation_roll_2))) false false)
    (if (>= (`KismetMathLibrary.Abs` (- (`self.InitKeyPitch`) _relativerotation_pitch)) 90.0)
      (`self.SetMetalCaseState` "NewEnumerator2"))))

(fn `SetMetalCaseState`
  (params (NewState :type "/Game/Blueprints/Gimmicks/EMetalCase Enum" :default "NewEnumerator0"))
  (bind _output_get (set `self.State` NewState))
  (switch `/Game/Blueprints/Gimmicks/EMetalCase` _output_get
    (:`NewEnumerator0`
      (`SceneComponent.SetVisibility` (`self.MeshKey`) false false)
      (`ActorComponent.SetActive` (`self.MeshKey`) false false)
      (`PrimitiveComponent.SetCollisionEnabled` (`self.KeyEnterArea`) "QueryOnly")
      (`PrimitiveComponent.SetCollisionEnabled` (`self.KeyGrabArea`) "NoCollision"))
    (:`NewEnumerator1`
      (`SceneComponent.SetVisibility` (`self.MeshKey`) true false)
      (`ActorComponent.SetActive` (`self.MeshKey`) true false)
      (`PrimitiveComponent.SetCollisionEnabled` (`self.KeyEnterArea`) "NoCollision")
      (`PrimitiveComponent.SetCollisionEnabled` (`self.KeyGrabArea`) "QueryOnly"))
    (:`NewEnumerator2`
      (`SceneComponent.SetVisibility` (`self.MeshKey`) true false)
      (`ActorComponent.SetActive` (`self.MeshKey`) true false)
      (`PrimitiveComponent.SetCollisionEnabled` (`self.KeyEnterArea`) "NoCollision")
      (`PrimitiveComponent.SetCollisionEnabled` (`self.KeyGrabArea`) "NoCollision"))))

(fn `UserConstructionScript`)