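; BP_TeleportArea is a teleport target that highlights itself while a teleport ray is on it.
; OnEnterTeleportRay shows the LightPoint, PointObject and PointObject2 components, and OnExitTeleportRay hides them.
; BeginPlay runs the same hide logic, so the highlight starts off invisible.
; The Blueprint handles only this visual feedback and contains no ray detection or teleport movement logic.
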(event `OnEnterTeleportRay`
  (`SceneComponent.SetVisibility` (`self.LightPoint`) true false)
  (`SceneComponent.SetVisibility` (`self.PointObject`) true false)
  (`SceneComponent.SetVisibility` (`self.PointObject2`) true false))

(event `OnExitTeleportRay`
  (`SceneComponent.SetVisibility` (`self.LightPoint`) false false :!label _label)
  (`SceneComponent.SetVisibility` (`self.PointObject`) false false)
  (`SceneComponent.SetVisibility` (`self.PointObject2`) false false))

(event `self.ReceiveBeginPlay`
  (goto _label))

(fn `UserConstructionScript`)