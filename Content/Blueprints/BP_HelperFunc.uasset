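; BP_HelperFunc is a set of helper functions for vector angle math and game mode access.
; Two functions return the angle between two vectors, in radians or degrees, as the arccosine of the dot product of their normalized inputs.
; A third gets the current game mode cast to BP_GameMode, with no handling for a failed cast.
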(fn `GetBPGameMode`
  (returns (NewParam :type "/Game/Blueprints/Managers/BP_GameMode Object Reference"))
  (bind _asbp_game_mode (cast `/Game/Blueprints/Managers/BP_GameMode` (`GameplayStatics.GetGameMode` null))
    (:`then`
      _)
    (:`CastFailed`
      _))
  (return _asbp_game_mode))

(fn `GetDegreeBetweenTwoVectors`
  (params (A :type "Vector Structure") (B :type "Vector Structure"))
  (returns (NewParam :type "Float (double-precision)"))
  (return (`KismetMathLibrary.DegAcos` (`KismetMathLibrary.Dot_VectorVector` (`KismetMathLibrary.Normal` A) (`KismetMathLibrary.Normal` B)))))

(fn `GetRadianBetweenTwoVectors`
  (params (A :type "Vector Structure") (B :type "Vector Structure"))
  (returns (NewParam :type "Float (double-precision)"))
  (return (`KismetMathLibrary.Acos` (`KismetMathLibrary.Dot_VectorVector` (`KismetMathLibrary.Normal` A) (`KismetMathLibrary.Normal` B)))))