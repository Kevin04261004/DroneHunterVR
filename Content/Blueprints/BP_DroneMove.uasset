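; BP_DroneMove is a Blueprint actor that travels along the spline of a referenced SplineBP, starting on BeginPlay.
; A MovingCart timeline, with play rate set to the inverse of Speed, drives a blend from zero to the full spline length.
; Each update sets the actor's world location and rotation from the spline at that distance, so Speed acts as a travel-time multiplier.
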(event `Move Cart`
  (bind _spline (`/Game/Blueprints/BP_Spline.Spline` (`self.SplineBP`)))
  (bind _returnvalue (`KismetMathLibrary.Lerp` 0.0 (`SplineComponent.GetSplineLength` (`/Game/Blueprints/BP_Spline.Spline` (`self.SplineBP`))) (`self.Blend`)))
  (`TimelineComponent.SetPlayRate` (`self.Moving Cart`) (/ 1.0 (`self.Speed`)))
  (bind (_direction _cart) (`Timeline|Moving Cart`)
    (:`Update`
      (set `self.Blend` _cart)
      (`self.K2_SetActorLocationAndRotation` (`SplineComponent.GetLocationAtDistanceAlongSpline` _spline _returnvalue "World") (`SplineComponent.GetRotationAtDistanceAlongSpline` _spline _returnvalue "World")))))

(event `self.ReceiveBeginPlay`
  (`self.Move Cart`))

(fn `UserConstructionScript`)