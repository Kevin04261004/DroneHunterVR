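; VR player pawn that spawns two BP_Hand actors, attaches itself to the BP_CartMove arrow and corrects camera height against PlayerStart after a delay.
; Enhanced Input drives hand grab/release, menu toggling and snap turns that pivot around the camera.
; Holding move line-traces from the right hand to highlight BP_TeleportArea actors, and releasing teleports there, compensating for headset offset.
; Inventory toggle and smooth movement exist but are unwired.
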(event `self.ReceiveBeginPlay`
  (bind (_returnvalue_x _returnvalue_y _returnvalue_z) (`KismetMathLibrary.BreakVector` (`SceneComponent.K2_GetComponentLocation` (`self.Camera`))))
  (`|ExecutionSequence`
    (:`then_0`
      (`EnhancedInputSubsystemInterface.AddMappingContext` (pcsubsystem `EnhancedInputLocalPlayerSubsystem` (`GameplayStatics.GetPlayerController` 0)) "/Game/Input/IMC_VR_Default.IMC_VR_Default" 0 (struct)))
    (:`then_1`
      (`HeadMountedDisplayFunctionLibrary.SetTrackingOrigin` "Local")
      (`KismetSystemLibrary.Delay` 1.0)
      (bind _returnvalue (`GameplayStatics.GetActorOfClass` "/Script/Engine.PlayerStart"))
      (`SceneComponent.K2_AddRelativeLocation` (`self.VRRoot`) (`KismetMathLibrary.MakeVector` 0.0 0.0 (- (+ (`self.DesiredCameraHeight`) (.z (.location (`self.GetTransform` _returnvalue)))) _returnvalue_z)) false false))
    (:`then_2`
      (bind _returnvalue_2 (`|SpawnActorFromClass` "/Game/Blueprints/BP_Hand.BP_Hand_C" (`KismetMathLibrary.MakeTransform` (0.0 0.0 0.0)) "Undefined" "OverrideRootScale" self true null))
      (bind _output_get (set `self.LeftHand` _returnvalue_2))
      (`self.K2_AttachToComponent` _output_get (`self.VRRoot`) "None" "SnapToTarget" "SnapToTarget" "KeepWorld" true))
    (:`then_3`
      (bind _returnvalue_3 (`|SpawnActorFromClass` "/Game/Blueprints/BP_Hand.BP_Hand_C" (`KismetMathLibrary.MakeTransform` (0.0 0.0 0.0)) "Undefined" "OverrideRootScale" self false null))
      (bind _output_get_2 (set `self.RightHand` _returnvalue_3))
      (`self.K2_AttachToComponent` _output_get_2 (`self.VRRoot`) "None" "SnapToTarget" "SnapToTarget" "KeepWorld" true))
    (:`then_4`
      (bind _returnvalue_4 (`GameplayStatics.GetActorOfClass` "/Game/Blueprints/BP_CartMove.BP_CartMove_C"))
      (bind _arrow (`/Game/Blueprints/BP_CartMove.Arrow` _returnvalue_4))
      (`self.K2_SetActorLocationAndRotation` (`SceneComponent.K2_GetComponentLocation` _arrow) (`SceneComponent.K2_GetComponentRotation` _arrow))
      (`self.K2_AttachToComponent` _arrow "None" "KeepWorld" "KeepWorld" "KeepWorld"))))

(event `EnhancedInput|/Game/Input/Actions/Hands/IA_VR_Menu_Toggle_Right`
  (params (ActionValue :type Boolean) (ElapsedSeconds :type "Float (double-precision)") (TriggeredSeconds :type "Float (double-precision)") (InputAction :type "InputAction Object Reference" :default "/Game/Input/Actions/Hands/IA_VR_Menu_Toggle_Right.IA_VR_Menu_Toggle_Right"))
  (:`Started`
    (`self.ToggleMenu`)))

(event `EnhancedInput|/Game/Input/Actions/IA_VR_Turn`
  (params (ActionValue :type "Float (double-precision)") (ElapsedSeconds :type "Float (double-precision)") (TriggeredSeconds :type "Float (double-precision)") (InputAction :type "InputAction Object Reference" :default "/Game/Input/Actions/IA_VR_Turn.IA_VR_Turn"))
  (:`Started`
    (`self.SnapTurn` (> ActionValue 0.0))))

(event `EnhancedInput|/Game/Input/Actions/IA_VR_Grab_Left`
  (params (ActionValue :type "Float (double-precision)") (ElapsedSeconds :type "Float (double-precision)") (TriggeredSeconds :type "Float (double-precision)") (InputAction :type "InputAction Object Reference" :default "/Game/Input/Actions/IA_VR_Grab_Left.IA_VR_Grab_Left"))
  (bind _lefthand (`self.LeftHand`))
  (:`Started`
    (`/Game/Blueprints/BP_Hand.HandleGrab` _lefthand :!label _label))
  (:`Ongoing`
    (goto _label))
  (:`Completed`
    (`/Game/Blueprints/BP_Hand.HandleRelease` _lefthand)))

(event `EnhancedInput|/Game/Input/Actions/IA_VR_Move`
  (params (ActionValue :type "Float (double-precision)") (ElapsedSeconds :type "Float (double-precision)") (TriggeredSeconds :type "Float (double-precision)") (InputAction :type "InputAction Object Reference" :default "/Game/Input/Actions/IA_VR_Move.IA_VR_Move"))
  (:`Started`
    (`self.StartTeleportTrace`)
    (`KismetSystemLibrary.PrintText` "Start"))
  (:`Completed`
    (`self.EndTeleportTrace`)
    (`KismetSystemLibrary.PrintText` "End")))

(event `EnhancedInput|/Game/Input/Actions/IA_VR_Grab_Right`
  (params (ActionValue :type "Float (double-precision)") (ElapsedSeconds :type "Float (double-precision)") (TriggeredSeconds :type "Float (double-precision)") (InputAction :type "InputAction Object Reference" :default "/Game/Input/Actions/IA_VR_Grab_Right.IA_VR_Grab_Right"))
  (bind _righthand (`self.RightHand`))
  (:`Started`
    (`/Game/Blueprints/BP_Hand.HandleGrab` _righthand))
  (:`Completed`
    (`/Game/Blueprints/BP_Hand.HandleRelease` _righthand)))

(event `self.ReceiveTick`
  (params (DeltaSeconds :type "Float (single-precision)"))
  (`self.UpdateTeleportTrace`))

(fn `EndTeleportTrace`
  (if (`self.bTeleportTrace`)
    (set `self.bTeleportTrace` false)
    (bind _teleportarea (`self.TeleportArea`)
      (:`then`
        (`/Game/Blueprints/Teleport/BP_TeleportArea.OnExitTeleportRay` _teleportarea)
        (`self.TryTeleport`)
        (set `self.TeleportArea` null))
      (:`else`))))

(fn `SnapTurn`
  (params (bRightTurn :type Boolean))
  (locals (LocalYawDelta :type "Float (double-precision)") (LocalPrevCameraLocation :type "Vector Structure"))
  (bind _snapturndegrees (`self.SnapTurnDegrees`))
  (set `local.LocalPrevCameraLocation` (`SceneComponent.K2_GetComponentLocation` (`self.Camera`)))
  (`self.K2_AddActorWorldRotation` (`KismetMathLibrary.MakeRotator` 0.0 0.0 (`KismetMathLibrary.SelectFloat` (`KismetMathLibrary.Abs` _snapturndegrees) _snapturndegrees (`local.bRightTurn`))) false true)
  (`self.K2_AddActorWorldOffset` (- (`local.LocalPrevCameraLocation`) (`SceneComponent.K2_GetComponentLocation` (`self.Camera`))) false true))

(fn `StartTeleportTrace`
  (set `self.bTeleportTrace` true))

(fn `ToggleInventory`
  (bind _camera (`self.Camera`))
  (bind _returnvalue (+ (`SceneComponent.K2_GetComponentLocation` _camera) (* (`SceneComponent.GetForwardVector` _camera) 50.0)))
  (bind _inventoryref (`self.InventoryRef`)
    (:`then`
      (`/Game/Blueprints/UI/BP_Inventory.OnCloseInventory` _inventoryref))
    (:`else`
      (bind _returnvalue_2 (`|SpawnActorFromClass` "/Game/Blueprints/UI/BP_Inventory.BP_Inventory_C" (`KismetMathLibrary.MakeTransform` _returnvalue (`KismetMathLibrary.FindLookAtRotation` _returnvalue (`SceneComponent.K2_GetComponentLocation` (`self.Camera`)))) "Undefined" "OverrideRootScale" null self))
      (bind _output_get (set `self.InventoryRef` _returnvalue_2))
      (`/Game/Blueprints/UI/BP_Inventory.OnOpenInventory` _output_get))))

(fn `ToggleMenu`
  (`self.MenuRef`
    (:`then`
      (`/Game/Blueprints/UI/BP_Menu.CloseMenu` (`self.MenuRef`)))
    (:`else`
      (bind _returnvalue (`|SpawnActorFromClass` "/Game/Blueprints/UI/BP_Menu.BP_Menu_C" (`KismetMathLibrary.MakeTransform` (0.0 0.0 0.0)) "Undefined" "OverrideRootScale" null self))
      (set `self.MenuRef` _returnvalue))))

(fn `TryTeleport`
  (bind (_returnvalue_roll _returnvalue_pitch _returnvalue_yaw) (`KismetMathLibrary.BreakRotator` (`self.K2_GetActorRotation`)))
  (bind (_returnvalue_x _returnvalue_y) (`KismetMathLibrary.BreakVector` (- (`SceneComponent.K2_GetComponentLocation` (`self.Camera`)) (`self.K2_GetActorLocation`))))
  (bind _teleportarea (`self.TeleportArea`)
    (:`then`
      (`self.K2_TeleportTo` (- (`self.K2_GetActorLocation` _teleportarea) (`KismetMathLibrary.MakeVector` _returnvalue_x _returnvalue_y)) (`KismetMathLibrary.MakeRotator` 0.0 0.0 _returnvalue_yaw))
      (bind _output_get (set `self.LastTeleportArea` _teleportarea))
      (`/Game/Blueprints/Teleport/BP_TeleportArea.OnExitTeleportRay` _output_get))
    (:`else`)))

(fn `UpdateTeleportTrace`
  (bind _returnvalue (`SceneComponent.K2_GetComponentLocation` (`/Game/Blueprints/BP_Hand.WidgetAimSocket` (`self.RightHand`))))
  (if (`self.bTeleportTrace`)
    (bind (_outhit _returnvalue_2) (`KismetSystemLibrary.LineTraceSingle` _returnvalue (+ _returnvalue (* (`SceneComponent.GetForwardVector` (`/Game/Blueprints/BP_Hand.WidgetAimSocket` (`self.RightHand`))) 3000.0)) "TraceTypeQuery4" false (`|MakeArray` (`self.LastTeleportArea`) :!type "Actor Object Reference") "ForOneFrame" true (struct :`R` 1.0 :`A` 1.0) (struct :`G` 1.0 :`A` 1.0) 1.0))
    (if _returnvalue_2
      (bind _asbp_teleport_area (cast `/Game/Blueprints/Teleport/BP_TeleportArea` (`.HitActor` (`GameplayStatics.BreakHitResult` _outhit))))
      (if (!= _asbp_teleport_area (`self.TeleportArea`))
        (bind _teleportarea (`self.TeleportArea`)
          (:`then`
            (`/Game/Blueprints/Teleport/BP_TeleportArea.OnExitTeleportRay` _teleportarea))
          (:`else`
            _))
        (set `self.TeleportArea` _asbp_teleport_area)
        (bind _teleportarea_2 (`self.TeleportArea`)
          (:`then`
            (`/Game/Blueprints/Teleport/BP_TeleportArea.OnEnterTeleportRay` _teleportarea_2))
          (:`else`)))
      (else
        (bind _teleportarea_3 (`self.TeleportArea`)
          (:`then`
            (`/Game/Blueprints/Teleport/BP_TeleportArea.OnExitTeleportRay` _teleportarea_3)
            (set `self.TeleportArea` null))
          (:`else`))))))

(fn `UserConstructionScript`)